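; GM_RunnerGameMode is the runner game's GameMode, which handles per-level background music.
; On BeginPlay it compares the current level name to Level1, Level2 and Level3, creates that level's 2D sound cue, stores the audio component and plays it.
; A FadeOut event fades the stored component to silence over a given duration.
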(event `self.ReceiveBeginPlay`
  (bind _returnvalue (`GameplayStatics.GetCurrentLevelName` true))
  (if (`KismetStringLibrary.EqualEqual_StrStr` _returnvalue "Level1")
    (bind _returnvalue_2 (`GameplayStatics.CreateSound2D` "/Game/Music/SAINT_PEPSI_-_Cherry_Pepsi_Cue.SAINT_PEPSI_-_Cherry_Pepsi_Cue" 1.0 1.0 0.0 null))
    (bind _output_get (set `self.AudioComponent` _returnvalue_2))
    (`AudioComponent.Play` _output_get 0.0)
    (elif (`KismetStringLibrary.EqualEqual_StrStr` _returnvalue "Level2")
      (bind _returnvalue_3 (`GameplayStatics.CreateSound2D` "/Game/Music/BLOODY_STREAM_-_JoJo_s_Bizarre_Adventure_OP_2__EUROBEAT_COVER___iTunesSpotify__Cue.BLOODY_STREAM_-_JoJo_s_Bizarre_Adventure_OP_2__EUROBEAT_COVER___iTunesSpotify__Cue" 1.0 1.0 0.0 null))
      (bind _output_get_2 (set `self.AudioComponent` _returnvalue_3))
      (`AudioComponent.Play` _output_get_2 0.0)
      (elif (`KismetStringLibrary.EqualEqual_StrStr` _returnvalue "Level3")
        (bind _returnvalue_4 (`GameplayStatics.CreateSound2D` "/Game/Music/Il_Vento_D_oro_Eurobeat_Remix_Cue.Il_Vento_D_oro_Eurobeat_Remix_Cue" 1.0 1.0 0.0 null))
        (bind _output_get_3 (set `self.AudioComponent` _returnvalue_4))
        (`AudioComponent.Play` _output_get_3 0.0)))))

(event `FadeOut`
  (params (Duration :type "Float (double-precision)"))
  (`AudioComponent.FadeOut` (`self.AudioComponent`) Duration 0.0))

(fn `UserConstructionScript`)