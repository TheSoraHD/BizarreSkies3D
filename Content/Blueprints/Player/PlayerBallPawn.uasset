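; PlayerBallPawn is a player ball pawn that travels forward automatically while the player steers it left and right.
; Tick advances the root component along world X by ForwardSpeed, and the MoveLeftRight axis shifts it along world Y by MouseSpeed.
; Both moves set world location directly, scaled by delta time, with no physics forces or movement component involved.
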(event `self.ReceiveTick`
  (params (DeltaSeconds :type "Float (single-precision)"))
  (bind (_returnvalue_x _returnvalue_y _returnvalue_z) (`KismetMathLibrary.BreakVector` (`SceneComponent.K2_GetComponentLocation` (`self.DefaultSceneRoot`))))
  (`SceneComponent.K2_SetWorldLocation` (`self.DefaultSceneRoot`) (`KismetMathLibrary.MakeVector` (+ (* DeltaSeconds (`self.ForwardSpeed`)) _returnvalue_x) _returnvalue_y _returnvalue_z) false false))

(event `InputAxis|MoveLeftRight`
  (params (AxisValue :type "Float (single-precision)"))
  (bind (_returnvalue_x _returnvalue_y _returnvalue_z) (`KismetMathLibrary.BreakVector` (`SceneComponent.K2_GetComponentLocation` (`self.DefaultSceneRoot`))))
  (`SceneComponent.K2_SetWorldLocation` (`self.DefaultSceneRoot`) (`KismetMathLibrary.MakeVector` _returnvalue_x (+ (* (* AxisValue (`GameplayStatics.GetWorldDeltaSeconds`)) (`self.MouseSpeed`)) _returnvalue_y) _returnvalue_z) false false))

(fn `UserConstructionScript`)