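; Player ball character for a runner that moves constantly forward along X and steers sideways with an input axis.
; Each Tick advances the capsule by forward speed plus an offset that acceleration and deceleration timelines drive.
; Tick also zeroes capsule rotation, clamps lateral position to a symmetric limit and pins camera height.
; The camera counters part of the sideways movement through its relative offset, and all movement sets world location directly.
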(event `self.ReceiveTick`
  (params (DeltaSeconds :type "Float (single-precision)"))
  (`self.ConstantRun`)
  (`self.FixedCameraHeightAndPlayerRotation`))

(event `InputAxis|MoveLeftRight`
  (params (AxisValue :type "Float (single-precision)"))
  (bind (_returnvalue_x _returnvalue_y _returnvalue_z) (`KismetMathLibrary.BreakVector` (`SceneComponent.K2_GetComponentLocation` (`self.CapsuleComponent`))))
  (`SceneComponent.K2_SetWorldLocation` (`self.CapsuleComponent`) (`KismetMathLibrary.MakeVector` _returnvalue_x (+ (* (* AxisValue (`GameplayStatics.GetWorldDeltaSeconds`)) (`self.MouseSpeed`)) _returnvalue_y) _returnvalue_z) false false))

(event `Acelerate`
  (bind (_direction _aceleration) (`Timeline|AcelerationTimeline` :!via `PlayFromStart`)
    (:`Update`
      (set `self.AcelerationSpeed` (* (* _aceleration (`self.AcelerationMultiplier`)) (`GameplayStatics.GetWorldDeltaSeconds`))))))

(event `Decelerate`
  (bind (_direction _aceleration) (`Timeline|Timeline_0` :!via `PlayFromStart`)
    (:`Update`
      (set `self.AcelerationSpeed` (* (* _aceleration (`self.DecelerationMultiplier`)) (`GameplayStatics.GetWorldDeltaSeconds`))))))

(fn `ConstantRun`
  (bind (_returnvalue_x _returnvalue_y _returnvalue_z) (`KismetMathLibrary.BreakVector` (`SceneComponent.K2_GetComponentLocation` (`self.CapsuleComponent`))))
  (`SceneComponent.K2_SetWorldLocation` (`self.CapsuleComponent`) (`KismetMathLibrary.MakeVector` (+ (+ (* (`GameplayStatics.GetWorldDeltaSeconds`) (`self.ForwardSpeed`)) (`self.AcelerationSpeed`)) _returnvalue_x) _returnvalue_y _returnvalue_z) false false))

(fn `FixedCameraHeightAndPlayerRotation`
  (locals (TempY :type "Float (double-precision)"))
  (bind _camera (`self.Camera`))
  (bind _camera_2 (`self.Camera`))
  (bind _capsulecomponent (`self.CapsuleComponent`))
  (bind (_returnvalue_x _returnvalue_y _returnvalue_z) (`KismetMathLibrary.BreakVector` (`SceneComponent.K2_GetComponentLocation` _capsulecomponent)))
  (bind (_returnvalue_x_2 _returnvalue_y_2) (`KismetMathLibrary.BreakVector` (`SceneComponent.K2_GetComponentLocation` (`self.CapsuleComponent`))))
  (bind (_returnvalue_x_3 _returnvalue_y_3) (`KismetMathLibrary.BreakVector` (`SceneComponent.K2_GetComponentLocation` _camera)))
  (bind (_relativelocation_x _relativelocation_y _relativelocation_z) (`KismetMathLibrary.BreakVector` (`SceneComponent.RelativeLocation` _camera_2)))
  (`SceneComponent.K2_SetWorldRotation` _capsulecomponent (`KismetMathLibrary.MakeRotator` 0.0) false false)
  (if (> (`KismetMathLibrary.Abs` _returnvalue_y) 700.0)
    (if (> _returnvalue_y 0.0)
      (set `local.TempY` 700.0)
      (else
        (set `local.TempY` -700.0)))
    (`SceneComponent.K2_SetWorldLocation` (`self.CapsuleComponent`) (`KismetMathLibrary.MakeVector` _returnvalue_x (`local.TempY`) _returnvalue_z) false false))
  ;[1 1 1] Camera
  (`SceneComponent.K2_SetRelativeLocation` _camera_2 (`KismetMathLibrary.MakeVector` _relativelocation_x (/ _returnvalue_y_2 -1.5) _relativelocation_z) false false)
  (`SceneComponent.K2_SetWorldLocation` _camera (`KismetMathLibrary.MakeVector` _returnvalue_x_3 _returnvalue_y_3 (`self.CameraHeight`)) false false))

(fn `UserConstructionScript`)