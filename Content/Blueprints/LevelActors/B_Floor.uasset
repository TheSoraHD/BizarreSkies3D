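; B_Floor is a level actor that builds a rectangular tiled floor from static mesh components.
; Its construction script runs nested inclusive loops over XTiles and YTiles, adding one mesh per grid cell at 100-unit spacing.
; When AutosetLocationInWorld is set, it moves the root in world space, shifting Y negatively by half the grid's width.
; The event graph has no active logic.
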(fn `UserConstructionScript`
  (for _index (range (+ (`self.XTiles`) 1))
    (for _index_2 (range (+ (`self.YTiles`) 1))
      (`AddComponent|NODE_AddStaticMeshComponent-0` :`RelativeTransform` (`KismetMathLibrary.MakeTransform` (`KismetMathLibrary.MakeVector` (* _index 100.0) (* _index_2 100.0))))))
  (if (`self.Autoset Location in World?`)
    (`SceneComponent.K2_SetWorldLocation` (`self.DefaultSceneRoot`) (`KismetMathLibrary.MakeVector` 0.0 (* (+ (`self.YTiles`) 1) -50.0)) false false)))