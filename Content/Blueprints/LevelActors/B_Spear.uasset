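; B_Spear is a level trap that extends a spear along negative relative X when the player ball enters its detection box.
; A timeline's GrowMultiplier, scaled by GrowingSpeed and delta time, gives a per-frame increment that moves tip and shaft while stretching the shaft's X scale.
; Player overlaps with either spear part only print a TO-DO, as killing the player is not implemented.
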(event `GrowSpear`
  (bind _speartip (`self.SpearTip`))
  (bind _spear (`self.Spear`))
  (bind (_relativelocation_x _relativelocation_y _relativelocation_z) (`KismetMathLibrary.BreakVector` (`SceneComponent.RelativeLocation` _speartip)))
  (bind (_relativelocation_x_2 _relativelocation_y_2 _relativelocation_z_2) (`KismetMathLibrary.BreakVector` (`SceneComponent.RelativeLocation` _spear)))
  (bind (_relativescale3d_x _relativescale3d_y _relativescale3d_z) (`KismetMathLibrary.BreakVector` (`SceneComponent.RelativeScale3D` _spear)))
  (bind (_direction _growmultiplier) (`Timeline|SpearTimeline`)
    (:`Update`
      (`self.CalculateGrow` _growmultiplier)
      (`SceneComponent.K2_SetRelativeLocation` _speartip (`KismetMathLibrary.MakeVector` (- _relativelocation_x (`self.TotalGrow`)) _relativelocation_y _relativelocation_z) false false)
      (`SceneComponent.K2_SetRelativeLocation` _spear (`KismetMathLibrary.MakeVector` (- _relativelocation_x_2 (`self.TotalGrow`)) _relativelocation_y_2 _relativelocation_z_2) false false)
      (`SceneComponent.SetRelativeScale3D` _spear (`KismetMathLibrary.MakeVector` (+ (* (`self.TotalGrow`) 0.003) _relativescale3d_x) _relativescale3d_y _relativescale3d_z)))))

(event `self.PlayerDetectionBox.OnComponentBeginOverlap`
  (params (OverlappedComponent :type "PrimitiveComponent Object Reference") (OtherActor :type "Actor Object Reference") (OtherComp :type "PrimitiveComponent Object Reference") (OtherBodyIndex :type Integer) (bFromSweep :type Boolean) (SweepResult :type "HitResult Structure (by ref)"))
  (cast `/Game/Blueprints/Player/PlayerBallCharacter` OtherActor)
  (`self.GrowSpear`))

(event `self.SpearTip.OnComponentBeginOverlap`
  (params (OverlappedComponent :type "PrimitiveComponent Object Reference") (OtherActor :type "Actor Object Reference") (OtherComp :type "PrimitiveComponent Object Reference") (OtherBodyIndex :type Integer) (bFromSweep :type Boolean) (SweepResult :type "HitResult Structure (by ref)"))
  (cast `/Game/Blueprints/Player/PlayerBallCharacter` OtherActor)
  (`KismetSystemLibrary.PrintString` "TO-DO: Kill player"))

(event `self.Spear.OnComponentBeginOverlap`
  (params (OverlappedComponent :type "PrimitiveComponent Object Reference") (OtherActor :type "Actor Object Reference") (OtherComp :type "PrimitiveComponent Object Reference") (OtherBodyIndex :type Integer) (bFromSweep :type Boolean) (SweepResult :type "HitResult Structure (by ref)"))
  (cast `/Game/Blueprints/Player/PlayerBallCharacter` OtherActor)
  (`KismetSystemLibrary.PrintString` "TO-DO: Kill player"))

(fn `UserConstructionScript`)