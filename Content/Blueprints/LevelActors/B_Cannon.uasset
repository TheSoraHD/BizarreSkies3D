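; B_Cannon is a level hazard that fires a bullet when the player ball enters its detection box.
; The overlap calls LaunchBullet, which plays a shot sound and runs a timeline, and also activates a particle effect that starts inactive.
; Each timeline update moves the bullet along negative relative Y, scaled by curve value, BulletSpeed and delta time.
; Touching either the bullet or the cannon itself triggers the player's Death.
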(event `self.ReceiveBeginPlay`
  (`ActorComponent.Deactivate` (`self.ParticleSystem`))
  (`ActorComponent.Deactivate` (`self.ParticleSystem1`)))

(event `LaunchBullet`
  (bind _bullet (`self.Bullet`))
  (bind (_relativelocation_x _relativelocation_y _relativelocation_z) (`KismetMathLibrary.BreakVector` (`SceneComponent.RelativeLocation` _bullet)))
  (`GameplayStatics.PlaySound2D` "/Game/SFX/Shoot_Cue.Shoot_Cue" 1.0 1.0 0.0 null null)
  (bind (_direction _locationmultiplier) (`Timeline|BulletTimeline`)
    (:`Update`
      (`SceneComponent.K2_SetRelativeLocation` _bullet (`KismetMathLibrary.MakeVector` _relativelocation_x (- _relativelocation_y (* (* _locationmultiplier (`self.BulletSpeed`)) (`GameplayStatics.GetWorldDeltaSeconds`))) _relativelocation_z) false false))))

(event `self.PlayerDetectionBox.OnComponentBeginOverlap`
  (params (OverlappedComponent :type "PrimitiveComponent Object Reference") (OtherActor :type "Actor Object Reference") (OtherComp :type "PrimitiveComponent Object Reference") (OtherBodyIndex :type Integer) (bFromSweep :type Boolean) (SweepResult :type "HitResult Structure (by ref)"))
  (cast `/Game/Blueprints/Player/PlayerBallCharacter` OtherActor)
  (`self.LaunchBullet`)
  (`ActorComponent.Activate` (`self.ParticleSystem`) true))

(event `self.Bullet.OnComponentBeginOverlap`
  (params (OverlappedComponent :type "PrimitiveComponent Object Reference") (OtherActor :type "Actor Object Reference") (OtherComp :type "PrimitiveComponent Object Reference") (OtherBodyIndex :type Integer) (bFromSweep :type Boolean) (SweepResult :type "HitResult Structure (by ref)"))
  (bind _asplayer_ball_character (cast `/Game/Blueprints/Player/PlayerBallCharacter` OtherActor))
  (`/Game/Blueprints/Player/PlayerBallCharacter.Death` _asplayer_ball_character))

(event `self.Cannon.OnComponentBeginOverlap`
  (params (OverlappedComponent :type "PrimitiveComponent Object Reference") (OtherActor :type "Actor Object Reference") (OtherComp :type "PrimitiveComponent Object Reference") (OtherBodyIndex :type Integer) (bFromSweep :type Boolean) (SweepResult :type "HitResult Structure (by ref)"))
  (bind _asplayer_ball_character (cast `/Game/Blueprints/Player/PlayerBallCharacter` OtherActor))
  (`/Game/Blueprints/Player/PlayerBallCharacter.Death` _asplayer_ball_character))

(fn `UserConstructionScript`)