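; B_Gate is a level trap actor whose gate moves when the player ball enters its detection box.
; The overlap calls GrowSpear, which plays a timeline that lowers the Gate's relative Z each update by a curve multiplier scaled by delta time and falling speed.
; Player contact with the Gate only prints a TO-DO for killing the player.
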(event `GrowSpear`
  (bind _gate (`self.Gate`))
  (bind (_relativelocation_x _relativelocation_y _relativelocation_z) (`KismetMathLibrary.BreakVector` (`SceneComponent.RelativeLocation` _gate)))
  (bind (_direction _heightmultiplier) (`Timeline|GateTimeline`)
    (:`Update`
      (`SceneComponent.K2_SetRelativeLocation` _gate (`KismetMathLibrary.MakeVector` _relativelocation_x _relativelocation_y (- _relativelocation_z (* (* _heightmultiplier (`GameplayStatics.GetWorldDeltaSeconds`)) (`self.FallingSpeed`)))) false false))))

(event `self.PlayerDetectionBox.OnComponentBeginOverlap`
  (params (OverlappedComponent :type "PrimitiveComponent Object Reference") (OtherActor :type "Actor Object Reference") (OtherComp :type "PrimitiveComponent Object Reference") (OtherBodyIndex :type Integer) (bFromSweep :type Boolean) (SweepResult :type "HitResult Structure (by ref)"))
  (cast `/Game/Blueprints/Player/PlayerBallCharacter` OtherActor)
  (`self.GrowSpear`))

(event `self.Gate.OnComponentBeginOverlap`
  (params (OverlappedComponent :type "PrimitiveComponent Object Reference") (OtherActor :type "Actor Object Reference") (OtherComp :type "PrimitiveComponent Object Reference") (OtherBodyIndex :type Integer) (bFromSweep :type Boolean) (SweepResult :type "HitResult Structure (by ref)"))
  (cast `/Game/Blueprints/Player/PlayerBallCharacter` OtherActor)
  (`KismetSystemLibrary.PrintString` "TO-DO: Kill player"))

(fn `UserConstructionScript`)