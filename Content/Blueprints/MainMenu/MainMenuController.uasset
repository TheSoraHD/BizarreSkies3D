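; Player controller for the main menu that creates the W_MainMenu widget on BeginPlay and shows it with the mouse cursor in game-and-UI input mode.
; Select, MenuLeft and MenuRight input actions forward to the widget's Start, MoveLeft and MoveRight functions, while Exit quits the game.
; Number keys 1 to 4 are hard-bound shortcuts that set the scalability quality level relative to max.
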(event `self.ReceiveBeginPlay`
  (bind _returnvalue (`|CreateWidget` "/Game/Blueprints/MainMenu/W_MainMenu.W_MainMenu_C"))
  (bind _output_get (set `self.MainMenu` _returnvalue))
  (`UserWidget.AddToViewport` _output_get 0)
  (`WidgetBlueprintLibrary.SetInputMode_GameAndUIEx` (`GameplayStatics.GetPlayerController` 0) _returnvalue "DoNotLock" false)
  (set `self.bShowMouseCursor` true))

(event `InputAction|Select`
  (params (Key :type "Key Structure"))
  (:`Pressed`
    (`/Game/Blueprints/MainMenu/W_MainMenu.Start` (`self.MainMenu`))))

(event `Key|One`
  (params (Key :type "Key Structure"))
  (:`Pressed`
    (`AutomationBlueprintFunctionLibrary.SetScalabilityQualityLevelRelativeToMax` 1)))

(event `Key|Two`
  (params (Key :type "Key Structure"))
  (:`Pressed`
    (`AutomationBlueprintFunctionLibrary.SetScalabilityQualityLevelRelativeToMax` 2)))

(event `InputAction|MenuLeft`
  (params (Key :type "Key Structure"))
  (:`Pressed`
    (`/Game/Blueprints/MainMenu/W_MainMenu.MoveLeft` (`self.MainMenu`))))

(event `Key|Three`
  (params (Key :type "Key Structure"))
  (:`Pressed`
    (`AutomationBlueprintFunctionLibrary.SetScalabilityQualityLevelRelativeToMax` 3)))

(event `Key|Four`
  (params (Key :type "Key Structure"))
  (:`Pressed`
    (`AutomationBlueprintFunctionLibrary.SetScalabilityQualityLevelRelativeToMax` 4)))

(event `InputAction|MenuRight`
  (params (Key :type "Key Structure"))
  (:`Pressed`
    (`/Game/Blueprints/MainMenu/W_MainMenu.MoveRight` (`self.MainMenu`))))

(event `InputAction|Exit`
  (params (Key :type "Key Structure"))
  (:`Pressed`
    (`KismetSystemLibrary.QuitGame` null "Quit")))

(fn `UserConstructionScript`)